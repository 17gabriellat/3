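; BP_SpawnForest is a forest spawner that adds scaled-down trees and flowers at random points inside its SpawnBox, with X clamped to a narrow band.
; SpawnTreeinForest checks GachaJenisPohon on BP_LahanUtama: type 1 spawns BP_TopViewType1 and saves the count to BPGI_Oxygen, while other types have no class set and skip saving.
; BeginPlay loads that count, and every fifth tree also spawns a random TipeFlower.
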(event Custom|Spawn%20Tree%20in%20Forest
  (bind _spawnbox (Variables|Default|GetSpawnBox))
  (bind _spawnbox_2 (Variables|Default|GetSpawnBox))
  (bind _returnvalue (Transformation|GetWorldLocation _spawnbox_2))
  (bind _returnvalue_2 (Transformation|GetWorldLocation _spawnbox))
  (bind _boxextent (Variables|/Script/Engine.BoxComponent|GetBoxExtent _spawnbox))
  (bind _boxextent_2 (Variables|/Script/Engine.BoxComponent|GetBoxExtent _spawnbox_2))
  (bind _returnvalue_3 (Math|Random|RandomPointinBoundingBox _returnvalue_2 _boxextent))
  (bind _returnvalue_4 (Math|Random|RandomPointinBoundingBox _returnvalue _boxextent_2))
  (bind _returnvalue_5 (Actor|GetActorOfClass "/Game/Lahan/BP_LahanUtama.BP_LahanUtama_C"))
  (if (== (Variables|/Game/Lahan/BP_LahanUtama.BP_LahanUtama_C|GetGacha%20Jenis%20Pohon _returnvalue_5) 1)
    (Game|SpawnActorfromClass "/Game/Tree/TreeType1/BP_TopViewType1.BP_TopViewType1_C" (Math|Transform|MakeTransform (Math|Vector|MakeVector (Math|Float|Clamp(Float) (.x _returnvalue_4) 1355.0 1375.0) (.y _returnvalue_4) (.z _returnvalue_4)) "0, 0, 0" "0.400000,0.400000,0.400000") "Undefined" "MultiplyWithRoot" 0 0)
    (Math|Integer|IncrementInt (Variables|Default|GetCount%20Tree)
      (:%20%20
        (CallFunction|SpawnFlower)
        (bind _asbpgi_oxygen (Utilities|Casting|CastToBPGI_Oxygen (Game|GetGameInstance)))
        (Variables|/Game/SaveGame/SG_SaveGame.SG_SaveGame_C|SetCountTreeSG (Variables|/Game/Tree/BPGI_Oxygen.BPGI_Oxygen_C|GetSG _asbpgi_oxygen) (Variables|Default|GetCount%20Tree))
        (Default|Save _asbpgi_oxygen)))
    (else
      (Game|SpawnActorfromClass "/Game/Tree/BP_TopViewType2.BP_TopViewType2_C" (Math|Transform|MakeTransform (Math|Vector|MakeVector (Math|Float|Clamp(Float) (.x _returnvalue_3) 1355.0 1375.0) (.y _returnvalue_3) (.z _returnvalue_3)) "0, 0, 0" "0.400000,0.400000,0.400000") "Undefined" "MultiplyWithRoot" 0 0)
      (Math|Integer|IncrementInt (Variables|Default|GetCount%20Tree)
        (:%20%20
          (CallFunction|SpawnFlower))))))

(event Custom|Spawn%20Flower
  (bind _spawnbox (Variables|Default|GetSpawnBox))
  (bind _returnvalue (Transformation|GetWorldLocation _spawnbox))
  (bind _boxextent (Variables|/Script/Engine.BoxComponent|GetBoxExtent _spawnbox))
  (bind _returnvalue_2 (Math|Random|RandomPointinBoundingBox _returnvalue _boxextent))
  ;[1 1 1] Spawn Flower Random Location
  (if (== (Math|Integer|%(Integer) (Variables|Default|GetCount%20Tree) 5) 0)
    (Game|SpawnActorfromClass (.OutItem (Utilities|Array|Random (Variables|Default|GetTipe%20Flower))) (Math|Transform|MakeTransform (Math|Vector|MakeVector (Math|Float|Clamp(Float) (.x _returnvalue_2) 1355.0 1375.0) (.y _returnvalue_2) (.z _returnvalue_2)) "90.000000,0.000000,0.000000" "1.000000,1.000000,1.000000") "Undefined" "MultiplyWithRoot" 0 0)))

(event Custom|InitializeConditionBefore)

(event EventBeginPlay
  (bind _asbpgi_oxygen (Utilities|Casting|CastToBPGI_Oxygen (Game|GetGameInstance)))
  (Variables|Default|SetCount%20Tree (Variables|/Game/SaveGame/SG_SaveGame.SG_SaveGame_C|GetCountTreeSG (Variables|/Game/Tree/BPGI_Oxygen.BPGI_Oxygen_C|GetSG _asbpgi_oxygen)))
  (CallFunction|InitializeConditionBefore))

(fn ConstructionScript)