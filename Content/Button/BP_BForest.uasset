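; BP_BForest is a controller that alternates a forest button between its day (Siang) and night (Malam) versions.
; On BeginPlay it finds the BP_LahanUtama actor and uses its Plane location, plus an offset, as the spawn point.
; ChangeButton spawns the day actor, swaps it for a rotated night actor after a fixed delay, then calls itself again to loop endlessly.
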(event Custom|Change%20Button
  ;[1 1 1] Change Button Siang dan Malam
  (bind _returnvalue (Game|SpawnActorfromClass "/Game/Button/BP_BForestSiang.BP_BForestSiang_C" (Math|Transform|MakeTransform (+ (Transformation|GetWorldLocation (Variables|/Game/Lahan/BP_LahanUtama.BP_LahanUtama_C|GetPlane (Variables|Default|GetRefLahan))) "-100.000000,-10.000000,200.000000") "0, 0, 0" "1.000000,1.000000,1.000000") "Undefined" "MultiplyWithRoot" 0 0))
  (Utilities|FlowControl|Delay 1e+01)
  (Actor|DestroyActor _returnvalue)
  (bind _returnvalue_2 (Game|SpawnActorfromClass "/Game/Button/BP_BForestMalam.BP_BForestMalam_C" (Math|Transform|MakeTransform (+ (Transformation|GetWorldLocation (Variables|/Game/Lahan/BP_LahanUtama.BP_LahanUtama_C|GetPlane (Variables|Default|GetRefLahan))) "-100.000000,-10.000000,200.000000") "0.000000,90.000000,0.000000" "1.000000,1.000000,1.000000") "Undefined" "MultiplyWithRoot" 0 0))
  (Utilities|FlowControl|Delay 1e+01)
  (Actor|DestroyActor _returnvalue_2)
  (CallFunction|ChangeButton))

(event EventBeginPlay
  (bind _returnvalue (Actor|GetActorOfClass "/Game/Lahan/BP_LahanUtama.BP_LahanUtama_C"))
  (Variables|Default|SetRefLahan _returnvalue)
  (CallFunction|ChangeButton))

(fn ConstructionScript)