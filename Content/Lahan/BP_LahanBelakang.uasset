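; Back land plot (LahanBelakang) that grows trees and produces oxygen in the game.
; NewTree spawns a tree in one of fourteen hard-coded slots, its type picked by BP_LahanUtama's GachaJenisPohon, and always tells BP_SpawnForest to add a forest tree.
; Past fourteen, only the count and forest keep growing.
; Once any tree exists, Tick disables itself and starts a one-second timer adding oxygen per tree to BPGI_Oxygen.
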(event Custom|New%20Tree
  (if (<= (Variables|Default|GetJumlah%20Pohon) 13)
    (bind _returnvalue (Actor|GetActorOfClass "/Game/Forest/BP_SpawnForest.BP_SpawnForest_C"))
    (Default|SpawnTreeinForest _returnvalue)
    (if (== (Variables|Default|GetJumlah%20Pohon) 0)
      (bind _returnvalue_2 (Actor|GetActorOfClass "/Game/Lahan/BP_LahanUtama.BP_LahanUtama_C"))
      (if (== (Variables|/Game/Lahan/BP_LahanUtama.BP_LahanUtama_C|GetGacha%20Jenis%20Pohon _returnvalue_2) 1)
        (Game|SpawnActorfromClass "/Game/Tree/TreeType1/BP_TreeType1LahanBelakang.BP_TreeType1LahanBelakang_C" (Math|Transform|MakeTransform "1060.000000,22210.000000,750.000000" "0, 0, 0" (Variables|Default|GetSpawn%20Transform%20Scale)) "Undefined" "MultiplyWithRoot" 0 0)
        (Math|Integer|IncrementInt (Variables|Default|GetJumlah%20Pohon))
        (else
          (Game|SpawnActorfromClass "/Game/Tree/BP_TreeType2LahanBelakang.BP_TreeType2LahanBelakang_C" (Math|Transform|MakeTransform "1060.000000,22220.000000,740.000000" "0, 0, 0" (Variables|Default|GetSpawn%20Transform%20Scale)) "Undefined" "MultiplyWithRoot" 0 0)
          (Math|Integer|IncrementInt (Variables|Default|GetJumlah%20Pohon)
            (:%20%20
              (Development|PrintString "Hello")))))
      (elif (== (Variables|Default|GetJumlah%20Pohon) 1)
        (bind _returnvalue_3 (Actor|GetActorOfClass "/Game/Lahan/BP_LahanUtama.BP_LahanUtama_C"))
        (if (== (Variables|/Game/Lahan/BP_LahanUtama.BP_LahanUtama_C|GetGacha%20Jenis%20Pohon _returnvalue_3) 1)
          (Game|SpawnActorfromClass "/Game/Tree/TreeType1/BP_TreeType1LahanBelakang.BP_TreeType1LahanBelakang_C" (Math|Transform|MakeTransform "1060.000000,22280.000000,720.000000" "0, 0, 0" (Variables|Default|GetSpawn%20Transform%20Scale)) "Undefined" "MultiplyWithRoot" 0 0)
          (Math|Integer|IncrementInt (Variables|Default|GetJumlah%20Pohon))
          (else
            (Game|SpawnActorfromClass "/Game/Tree/BP_TreeType2LahanBelakang.BP_TreeType2LahanBelakang_C" (Math|Transform|MakeTransform "1060.000000,22280.000000,710.000000" "0, 0, 0" (Variables|Default|GetSpawn%20Transform%20Scale)) "Undefined" "MultiplyWithRoot" 0 0)
            (Math|Integer|IncrementInt (Variables|Default|GetJumlah%20Pohon))))
        (elif (== (Variables|Default|GetJumlah%20Pohon) 2)
          (bind _returnvalue_4 (Actor|GetActorOfClass "/Game/Lahan/BP_LahanUtama.BP_LahanUtama_C"))
          (if (== (Variables|/Game/Lahan/BP_LahanUtama.BP_LahanUtama_C|GetGacha%20Jenis%20Pohon _returnvalue_4) 1)
            (Game|SpawnActorfromClass "/Game/Tree/TreeType1/BP_TreeType1LahanBelakang.BP_TreeType1LahanBelakang_C" (Math|Transform|MakeTransform "1060.000000,22350.000000,750.000000" "0, 0, 0" (Variables|Default|GetSpawn%20Transform%20Scale)) "Undefined" "MultiplyWithRoot" 0 0)
            (Math|Integer|IncrementInt (Variables|Default|GetJumlah%20Pohon))
            (else
              (Game|SpawnActorfromClass "/Game/Tree/BP_TreeType2LahanBelakang.BP_TreeType2LahanBelakang_C" (Math|Transform|MakeTransform "1060.000000,22350.000000,740.000000" "0, 0, 0" (Variables|Default|GetSpawn%20Transform%20Scale)) "Undefined" "MultiplyWithRoot" 0 0)
              (Math|Integer|IncrementInt (Variables|Default|GetJumlah%20Pohon))))
          (elif (== (Variables|Default|GetJumlah%20Pohon) 3)
            (bind _returnvalue_5 (Actor|GetActorOfClass "/Game/Lahan/BP_LahanUtama.BP_LahanUtama_C"))
            (if (== (Variables|/Game/Lahan/BP_LahanUtama.BP_LahanUtama_C|GetGacha%20Jenis%20Pohon _returnvalue_5) 1)
              (Game|SpawnActorfromClass "/Game/Tree/TreeType1/BP_TreeType1LahanBelakang.BP_TreeType1LahanBelakang_C" (Math|Transform|MakeTransform "1060.000000,22420.000000,720.000000" "0, 0, 0" (Variables|Default|GetSpawn%20Transform%20Scale)) "Undefined" "MultiplyWithRoot" 0 0)
              (Math|Integer|IncrementInt (Variables|Default|GetJumlah%20Pohon))
              (else
                (Game|SpawnActorfromClass "/Game/Tree/BP_TreeType2LahanBelakang.BP_TreeType2LahanBelakang_C" (Math|Transform|MakeTransform "1060.000000,22420.000000,710.000000" "0, 0, 0" (Variables|Default|GetSpawn%20Transform%20Scale)) "Undefined" "MultiplyWithRoot" 0 0)
                (Math|Integer|IncrementInt (Variables|Default|GetJumlah%20Pohon))))
            (elif (== (Variables|Default|GetJumlah%20Pohon) 4)
              (bind _returnvalue_6 (Actor|GetActorOfClass "/Game/Lahan/BP_LahanUtama.BP_LahanUtama_C"))
              (if (== (Variables|/Game/Lahan/BP_LahanUtama.BP_LahanUtama_C|GetGacha%20Jenis%20Pohon _returnvalue_6) 1)
                (Game|SpawnActorfromClass "/Game/Tree/TreeType1/BP_TreeType1LahanBelakang.BP_TreeType1LahanBelakang_C" (Math|Transform|MakeTransform "1060.000000,22490.000000,750.000000" "0, 0, 0" (Variables|Default|GetSpawn%20Transform%20Scale)) "Undefined" "MultiplyWithRoot" 0 0)
                (Math|Integer|IncrementInt (Variables|Default|GetJumlah%20Pohon))
                (else
                  (Game|SpawnActorfromClass "/Game/Tree/BP_TreeType2LahanBelakang.BP_TreeType2LahanBelakang_C" (Math|Transform|MakeTransform "1060.000000,22490.000000,730.000000" "0, 0, 0" (Variables|Default|GetSpawn%20Transform%20Scale)) "Undefined" "MultiplyWithRoot" 0 0)
                  (Math|Integer|IncrementInt (Variables|Default|GetJumlah%20Pohon))))
              (elif (== (Variables|Default|GetJumlah%20Pohon) 5)
                (bind _returnvalue_7 (Actor|GetActorOfClass "/Game/Lahan/BP_LahanUtama.BP_LahanUtama_C"))
                (if (== (Variables|/Game/Lahan/BP_LahanUtama.BP_LahanUtama_C|GetGacha%20Jenis%20Pohon _returnvalue_7) 1)
                  (Game|SpawnActorfromClass "/Game/Tree/TreeType1/BP_TreeType1LahanBelakang.BP_TreeType1LahanBelakang_C" (Math|Transform|MakeTransform "1060.000000,22560.000000,720.000000" "0, 0, 0" (Variables|Default|GetSpawn%20Transform%20Scale)) "Undefined" "MultiplyWithRoot" 0 0)
                  (Math|Integer|IncrementInt (Variables|Default|GetJumlah%20Pohon))
                  (else
                    (Game|SpawnActorfromClass "/Game/Tree/BP_TreeType2LahanBelakang.BP_TreeType2LahanBelakang_C" (Math|Transform|MakeTransform "1060.000000,22560.000000,710.000000" "0, 0, 0" (Variables|Default|GetSpawn%20Transform%20Scale)) "Undefined" "MultiplyWithRoot" 0 0)
                    (Math|Integer|IncrementInt (Variables|Default|GetJumlah%20Pohon))))
                (elif (== (Variables|Default|GetJumlah%20Pohon) 6)
                  (bind _returnvalue_8 (Actor|GetActorOfClass "/Game/Lahan/BP_LahanUtama.BP_LahanUtama_C"))
                  (if (== (Variables|/Game/Lahan/BP_LahanUtama.BP_LahanUtama_C|GetGacha%20Jenis%20Pohon _returnvalue_8) 1)
                    (Game|SpawnActorfromClass "/Game/Tree/TreeType1/BP_TreeType1LahanBelakang.BP_TreeType1LahanBelakang_C" (Math|Transform|MakeTransform "1060.000000,22630.000000,750.000000" "0, 0, 0" (Variables|Default|GetSpawn%20Transform%20Scale)) "Undefined" "MultiplyWithRoot" 0 0)
                    (Math|Integer|IncrementInt (Variables|Default|GetJumlah%20Pohon))
                    (else
                      (Game|SpawnActorfromClass "/Game/Tree/BP_TreeType2LahanBelakang.BP_TreeType2LahanBelakang_C" (Math|Transform|MakeTransform "1060.000000,22620.000000,740.000000" "0, 0, 0" (Variables|Default|GetSpawn%20Transform%20Scale)) "Undefined" "MultiplyWithRoot" 0 0)
                      (Math|Integer|IncrementInt (Variables|Default|GetJumlah%20Pohon))))
                  (elif (== (Variables|Default|GetJumlah%20Pohon) 7)
                    (bind _returnvalue_9 (Actor|GetActorOfClass "/Game/Lahan/BP_LahanUtama.BP_LahanUtama_C"))
                    (if (== (Variables|/Game/Lahan/BP_LahanUtama.BP_LahanUtama_C|GetGacha%20Jenis%20Pohon _returnvalue_9) 1)
                      (Game|SpawnActorfromClass "/Game/Tree/TreeType1/BP_TreeType1LahanBelakang.BP_TreeType1LahanBelakang_C" (Math|Transform|MakeTransform "1060.000000,22210.000000,640.000000" "0, 0, 0" (Variables|Default|GetSpawn%20Transform%20Scale)) "Undefined" "MultiplyWithRoot" 0 0)
                      (Math|Integer|IncrementInt (Variables|Default|GetJumlah%20Pohon))
                      (else
                        (Game|SpawnActorfromClass "/Game/Tree/BP_TreeType2LahanBelakang.BP_TreeType2LahanBelakang_C" (Math|Transform|MakeTransform "1060.000000,22220.000000,630.000000" "0, 0, 0" (Variables|Default|GetSpawn%20Transform%20Scale)) "Undefined" "MultiplyWithRoot" 0 0)
                        (Math|Integer|IncrementInt (Variables|Default|GetJumlah%20Pohon))))
                    (elif (== (Variables|Default|GetJumlah%20Pohon) 8)
                      (bind _returnvalue_10 (Actor|GetActorOfClass "/Game/Lahan/BP_LahanUtama.BP_LahanUtama_C"))
                      (if (== (Variables|/Game/Lahan/BP_LahanUtama.BP_LahanUtama_C|GetGacha%20Jenis%20Pohon _returnvalue_10) 1)
                        (Game|SpawnActorfromClass "/Game/Tree/TreeType1/BP_TreeType1LahanBelakang.BP_TreeType1LahanBelakang_C" (Math|Transform|MakeTransform "1060.000000,22290.000000,610.000000" "0, 0, 0" (Variables|Default|GetSpawn%20Transform%20Scale)) "Undefined" "MultiplyWithRoot" 0 0)
                        (Math|Integer|IncrementInt (Variables|Default|GetJumlah%20Pohon))
                        (else
                          (Game|SpawnActorfromClass "/Game/Tree/BP_TreeType2LahanBelakang.BP_TreeType2LahanBelakang_C" (Math|Transform|MakeTransform "1060.000000,22290.000000,600.000000" "0, 0, 0" (Variables|Default|GetSpawn%20Transform%20Scale)) "Undefined" "MultiplyWithRoot" 0 0)
                          (Math|Integer|IncrementInt (Variables|Default|GetJumlah%20Pohon))))
                      (elif (== (Variables|Default|GetJumlah%20Pohon) 9)
                        (bind _returnvalue_11 (Actor|GetActorOfClass "/Game/Lahan/BP_LahanUtama.BP_LahanUtama_C"))
                        (if (== (Variables|/Game/Lahan/BP_LahanUtama.BP_LahanUtama_C|GetGacha%20Jenis%20Pohon _returnvalue_11) 1)
                          (Game|SpawnActorfromClass "/Game/Tree/TreeType1/BP_TreeType1LahanBelakang.BP_TreeType1LahanBelakang_C" (Math|Transform|MakeTransform "1060.000000,22350.000000,640.000000" "0, 0, 0" (Variables|Default|GetSpawn%20Transform%20Scale)) "Undefined" "MultiplyWithRoot" 0 0)
                          (Math|Integer|IncrementInt (Variables|Default|GetJumlah%20Pohon))
                          (else
                            (Game|SpawnActorfromClass "/Game/Tree/BP_TreeType2LahanBelakang.BP_TreeType2LahanBelakang_C" (Math|Transform|MakeTransform "1060.000000,22350.000000,630.000000" "0, 0, 0" (Variables|Default|GetSpawn%20Transform%20Scale)) "Undefined" "MultiplyWithRoot" 0 0)
                            (Math|Integer|IncrementInt (Variables|Default|GetJumlah%20Pohon))))
                        (elif (== (Variables|Default|GetJumlah%20Pohon) 10)
                          (bind _returnvalue_12 (Actor|GetActorOfClass "/Game/Lahan/BP_LahanUtama.BP_LahanUtama_C"))
                          (if (== (Variables|/Game/Lahan/BP_LahanUtama.BP_LahanUtama_C|GetGacha%20Jenis%20Pohon _returnvalue_12) 1)
                            (Game|SpawnActorfromClass "/Game/Tree/TreeType1/BP_TreeType1LahanBelakang.BP_TreeType1LahanBelakang_C" (Math|Transform|MakeTransform "1060.000000,22420.000000,610.000000" "0, 0, 0" (Variables|Default|GetSpawn%20Transform%20Scale)) "Undefined" "MultiplyWithRoot" 0 0)
                            (Math|Integer|IncrementInt (Variables|Default|GetJumlah%20Pohon))
                            (else
                              (Game|SpawnActorfromClass "/Game/Tree/BP_TreeType2LahanBelakang.BP_TreeType2LahanBelakang_C" (Math|Transform|MakeTransform "1060.000000,22420.000000,590.000000" "0, 0, 0" (Variables|Default|GetSpawn%20Transform%20Scale)) "Undefined" "MultiplyWithRoot" 0 0)
                              (Math|Integer|IncrementInt (Variables|Default|GetJumlah%20Pohon))))
                          (elif (== (Variables|Default|GetJumlah%20Pohon) 11)
                            (bind _returnvalue_13 (Actor|GetActorOfClass "/Game/Lahan/BP_LahanUtama.BP_LahanUtama_C"))
                            (if (== (Variables|/Game/Lahan/BP_LahanUtama.BP_LahanUtama_C|GetGacha%20Jenis%20Pohon _returnvalue_13) 1)
                              (Game|SpawnActorfromClass "/Game/Tree/TreeType1/BP_TreeType1LahanBelakang.BP_TreeType1LahanBelakang_C" (Math|Transform|MakeTransform "1060.000000,22490.000000,640.000000" "0, 0, 0" (Variables|Default|GetSpawn%20Transform%20Scale)) "Undefined" "MultiplyWithRoot" 0 0)
                              (Math|Integer|IncrementInt (Variables|Default|GetJumlah%20Pohon))
                              (else
                                (Game|SpawnActorfromClass "/Game/Tree/BP_TreeType2LahanBelakang.BP_TreeType2LahanBelakang_C" (Math|Transform|MakeTransform "1060.000000,22490.000000,620.000000" "0, 0, 0" (Variables|Default|GetSpawn%20Transform%20Scale)) "Undefined" "MultiplyWithRoot" 0 0)
                                (Math|Integer|IncrementInt (Variables|Default|GetJumlah%20Pohon))))
                            (elif (== (Variables|Default|GetJumlah%20Pohon) 12)
                              (bind _returnvalue_14 (Actor|GetActorOfClass "/Game/Lahan/BP_LahanUtama.BP_LahanUtama_C"))
                              (if (== (Variables|/Game/Lahan/BP_LahanUtama.BP_LahanUtama_C|GetGacha%20Jenis%20Pohon _returnvalue_14) 1)
                                (Game|SpawnActorfromClass "/Game/Tree/TreeType1/BP_TreeType1LahanBelakang.BP_TreeType1LahanBelakang_C" (Math|Transform|MakeTransform "1060.000000,22560.000000,610.000000" "0, 0, 0" (Variables|Default|GetSpawn%20Transform%20Scale)) "Undefined" "MultiplyWithRoot" 0 0)
                                (Math|Integer|IncrementInt (Variables|Default|GetJumlah%20Pohon))
                                (else
                                  (Game|SpawnActorfromClass "/Game/Tree/BP_TreeType2LahanBelakang.BP_TreeType2LahanBelakang_C" (Math|Transform|MakeTransform "1060.000000,22560.000000,590.000000" "0, 0, 0" (Variables|Default|GetSpawn%20Transform%20Scale)) "Undefined" "MultiplyWithRoot" 0 0)
                                  (Math|Integer|IncrementInt (Variables|Default|GetJumlah%20Pohon))))
                              (elif (== (Variables|Default|GetJumlah%20Pohon) 13)
                                (bind _returnvalue_15 (Actor|GetActorOfClass "/Game/Lahan/BP_LahanUtama.BP_LahanUtama_C"))
                                (if (== (Variables|/Game/Lahan/BP_LahanUtama.BP_LahanUtama_C|GetGacha%20Jenis%20Pohon _returnvalue_15) 1)
                                  (Game|SpawnActorfromClass "/Game/Tree/TreeType1/BP_TreeType1LahanBelakang.BP_TreeType1LahanBelakang_C" (Math|Transform|MakeTransform "1060.000000,22630.000000,640.000000" "0, 0, 0" (Variables|Default|GetSpawn%20Transform%20Scale)) "Undefined" "MultiplyWithRoot" 0 0)
                                  (Math|Integer|IncrementInt (Variables|Default|GetJumlah%20Pohon))
                                  (else
                                    (Game|SpawnActorfromClass "/Game/Tree/BP_TreeType2LahanBelakang.BP_TreeType2LahanBelakang_C" (Math|Transform|MakeTransform "1060.000000,22630.000000,620.000000" "0, 0, 0" (Variables|Default|GetSpawn%20Transform%20Scale)) "Undefined" "MultiplyWithRoot" 0 0)
                                    (Math|Integer|IncrementInt (Variables|Default|GetJumlah%20Pohon))))))))))))))))))
    (else
      (Math|Integer|IncrementInt (Variables|Default|GetJumlah%20Pohon)
        (:%20%20
          (bind _returnvalue_16 (Actor|GetActorOfClass "/Game/Forest/BP_SpawnForest.BP_SpawnForest_C"))
          (Default|SpawnTreeinForest _returnvalue_16))))))

(event Custom|Get%20Free%20O2
  (bind _asbpgi_oxygen (Utilities|Casting|CastToBPGI_Oxygen (Game|GetGameInstance)))
  (Variables|/Game/Tree/BPGI_Oxygen.BPGI_Oxygen_C|SetOxygen _asbpgi_oxygen (+ (Variables|/Game/Tree/BPGI_Oxygen.BPGI_Oxygen_C|GetOxygen _asbpgi_oxygen) (* (Variables|Default|GetJumlah%20Pohon) 6))))

(event EventTick
  (params (DeltaSeconds :type Float%20%28single-precision%29))
  (if (> (Variables|Default|GetJumlah%20Pohon) 0)
    (Actor|Tick|SetActorTickEnabled false)
    (Utilities|Time|SetTimerbyEvent (delegate Custom|Get%20Free%20O2) 1.0 true)))

(fn ConstructionScript)