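; BP_Forest is a forest actor that tracks planted trees and turns them into a passive oxygen income.
; NewTree spawns an actor at a fixed, half-scale transform and increments the tree count (JumlahPohon).
; Once the count is positive, Tick disables itself and starts a looping one-second timer.
; Each timer firing adds oxygen proportional to the tree count to the BPGI_Oxygen game instance.
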(event Custom|New%20Tree
  (Game|SpawnActorfromClass "/Game/Tree/BP_Tree6.BP_Tree6_C" (Math|Transform|MakeTransform "1290.000000,22270.000000,0.000000" "0, 0, 0" "0.500000,0.500000,0.500000") "Undefined" "MultiplyWithRoot" 0 0)
  (Math|Integer|IncrementInt (Variables|Default|GetJumlah%20Pohon)))

(event Custom|Get%20Free%20O2
  (bind _asbpgi_oxygen (Utilities|Casting|CastToBPGI_Oxygen (Game|GetGameInstance)))
  (Variables|/Game/Tree/BPGI_Oxygen.BPGI_Oxygen_C|SetOxygen _asbpgi_oxygen (+ (Variables|/Game/Tree/BPGI_Oxygen.BPGI_Oxygen_C|GetOxygen _asbpgi_oxygen) (* (Variables|Default|GetJumlah%20Pohon) 6))))

(event EventTick
  (params (DeltaSeconds :type Float%20%28single-precision%29))
  (if (> (Variables|Default|GetJumlah%20Pohon) 0)
    (Actor|Tick|SetActorTickEnabled false)
    (Utilities|Time|SetTimerbyEvent (delegate Custom|Get%20Free%20O2) 1.0 true)))

(fn ConstructionScript)