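; BP_LahanUtama is the main land plot, growing a dead tree through five upgrade stages paid with Oxygen from BPGI_Oxygen.
; Tick polls LevelTree and Oxygen, spawns a BP_BUpgrade button when affordable, and treats its disappearance as purchase, deducting PriceO2 and swapping tree actors.
; At full growth it spawns BP_BNewTree; once that is gone with Buy set, it calls NewTree on BP_LahanBelakang and resets to a dead tree.
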(event Custom|Beli%20Pohon%20Baru
  (bind _asbpgi_oxygen (Utilities|Casting|CastToBPGI_Oxygen (Game|GetGameInstance)))
  (Variables|Default|SetCan%20Buy%20a%20Tree? (and (== (Variables|Default|GetLevel%20Tree) 6) (>= (Variables|/Game/Tree/BPGI_Oxygen.BPGI_Oxygen_C|GetOxygen _asbpgi_oxygen) 1e+02))))

(event Custom|Upgrade%20Tree
  (Game|SpawnActorfromClass "/Game/Button/BP_BUpgrade.BP_BUpgrade_C" (Math|Transform|MakeTransform "1360.000000,22250.000000,110.000000" "0, 0, 0" "1.000000,1.000000,1.000000") "Undefined" "MultiplyWithRoot" 0 0)
  (Variables|Default|SetSpawn%20Upgrade%20Tree true))

(event EventBeginPlay
  (Game|SpawnActorfromClass "/Game/Tree/BP_DeadTree.BP_DeadTree_C" (Math|Transform|MakeTransform (Variables|Default|GetLocation%20Spawn) "0, 0, 0" "1.000000,1.000000,1.000000") "Undefined" "MultiplyWithRoot" 0 0)
  (Variables|Default|SetLevel%20Tree 1))

(event EventTick
  (params (DeltaSeconds :type Float%20%28single-precision%29))
  (if (== (Variables|Default|GetLevel%20Tree) 1)
    (bind _asbpgi_oxygen (Utilities|Casting|CastToBPGI_Oxygen (Game|GetGameInstance)))
    (if (>= (Variables|/Game/Tree/BPGI_Oxygen.BPGI_Oxygen_C|GetOxygen _asbpgi_oxygen) (Variables|Default|GetPrice%20O2))
      (bind _output_get (Variables|Default|SetUpgrade? true))
      (if (and _output_get (== (Variables|Default|GetSpawn%20Upgrade%20Tree) false))
        (CallFunction|UpgradeTree)
        (else
          (bind _returnvalue (Actor|GetActorOfClass "/Game/Button/BP_BUpgrade.BP_BUpgrade_C"))
          (Utilities|IsValid _returnvalue
            (:Is%20Not%20Valid
              (bind _asbpgi_oxygen_2 (Utilities|Casting|CastToBPGI_Oxygen (Game|GetGameInstance)))
              (Variables|/Game/Tree/BPGI_Oxygen.BPGI_Oxygen_C|SetOxygen _asbpgi_oxygen_2 (- (Variables|/Game/Tree/BPGI_Oxygen.BPGI_Oxygen_C|GetOxygen _asbpgi_oxygen_2) (Variables|Default|GetPrice%20O2)))
              (bind _returnvalue_2 (Actor|GetActorOfClass "/Game/Tree/BP_DeadTree.BP_DeadTree_C"))
              (Actor|DestroyActor _returnvalue_2)
              (Game|SpawnActorfromClass "/Game/Tree/BP_Tree1.BP_Tree1_C" (Math|Transform|MakeTransform (Variables|Default|GetLocation%20Spawn) "0, 0, 0" "1.000000,1.000000,1.000000") "Undefined" "MultiplyWithRoot" 0 0)
              (Variables|Default|SetLevel%20Tree 2)
              (Variables|Default|SetSpawn%20Upgrade%20Tree false))))))
    (elif (== (Variables|Default|GetLevel%20Tree) 2)
      (bind _asbpgi_oxygen_3 (Utilities|Casting|CastToBPGI_Oxygen (Game|GetGameInstance)))
      (if (>= (Variables|/Game/Tree/BPGI_Oxygen.BPGI_Oxygen_C|GetOxygen _asbpgi_oxygen_3) (Variables|Default|GetPrice%20O2))
        (bind _output_get_2 (Variables|Default|SetUpgrade? true))
        (if (and _output_get_2 (== (Variables|Default|GetSpawn%20Upgrade%20Tree) false))
          (CallFunction|UpgradeTree)
          (else
            (bind _returnvalue_3 (Actor|GetActorOfClass "/Game/Button/BP_BUpgrade.BP_BUpgrade_C"))
            (Utilities|IsValid _returnvalue_3
              (:Is%20Not%20Valid
                (bind _asbpgi_oxygen_4 (Utilities|Casting|CastToBPGI_Oxygen (Game|GetGameInstance)))
                (Variables|/Game/Tree/BPGI_Oxygen.BPGI_Oxygen_C|SetOxygen _asbpgi_oxygen_4 (- (Variables|/Game/Tree/BPGI_Oxygen.BPGI_Oxygen_C|GetOxygen _asbpgi_oxygen_4) (Variables|Default|GetPrice%20O2)))
                (bind _returnvalue_4 (Actor|GetActorOfClass "/Game/Tree/BP_Tree1.BP_Tree1_C"))
                (Actor|DestroyActor _returnvalue_4)
                (Game|SpawnActorfromClass "/Game/Tree/BP_Tree2.BP_Tree2_C" (Math|Transform|MakeTransform (Variables|Default|GetLocation%20Spawn) "0, 0, 0" "1.000000,1.000000,1.000000") "Undefined" "MultiplyWithRoot" 0 0)
                (Variables|Default|SetLevel%20Tree 3)
                (Variables|Default|SetSpawn%20Upgrade%20Tree false))))))
      (elif (== (Variables|Default|GetLevel%20Tree) 3)
        (bind _asbpgi_oxygen_5 (Utilities|Casting|CastToBPGI_Oxygen (Game|GetGameInstance)))
        (if (>= (Variables|/Game/Tree/BPGI_Oxygen.BPGI_Oxygen_C|GetOxygen _asbpgi_oxygen_5) (Variables|Default|GetPrice%20O2))
          (bind _output_get_3 (Variables|Default|SetUpgrade? true))
          (if (and _output_get_3 (== (Variables|Default|GetSpawn%20Upgrade%20Tree) false))
            (CallFunction|UpgradeTree)
            (else
              (bind _returnvalue_5 (Actor|GetActorOfClass "/Game/Button/BP_BUpgrade.BP_BUpgrade_C"))
              (Utilities|IsValid _returnvalue_5
                (:Is%20Not%20Valid
                  (bind _asbpgi_oxygen_6 (Utilities|Casting|CastToBPGI_Oxygen (Game|GetGameInstance)))
                  (Variables|/Game/Tree/BPGI_Oxygen.BPGI_Oxygen_C|SetOxygen _asbpgi_oxygen_6 (- (Variables|/Game/Tree/BPGI_Oxygen.BPGI_Oxygen_C|GetOxygen _asbpgi_oxygen_6) (Variables|Default|GetPrice%20O2)))
                  (bind _returnvalue_6 (Actor|GetActorOfClass "/Game/Tree/BP_Tree2.BP_Tree2_C"))
                  (Actor|DestroyActor _returnvalue_6)
                  (Game|SpawnActorfromClass "/Game/Tree/BP_Tree3.BP_Tree3_C" (Math|Transform|MakeTransform (Variables|Default|GetLocation%20Spawn) "0, 0, 0" "1.000000,1.000000,1.000000") "Undefined" "MultiplyWithRoot" 0 0)
                  (Variables|Default|SetLevel%20Tree 4)
                  (Variables|Default|SetSpawn%20Upgrade%20Tree false))))))
        (elif (== (Variables|Default|GetLevel%20Tree) 4)
          (bind _asbpgi_oxygen_7 (Utilities|Casting|CastToBPGI_Oxygen (Game|GetGameInstance)))
          (if (>= (Variables|/Game/Tree/BPGI_Oxygen.BPGI_Oxygen_C|GetOxygen _asbpgi_oxygen_7) (Variables|Default|GetPrice%20O2))
            (bind _output_get_4 (Variables|Default|SetUpgrade? true))
            (if (and _output_get_4 (== (Variables|Default|GetSpawn%20Upgrade%20Tree) false))
              (CallFunction|UpgradeTree)
              (else
                (bind _returnvalue_7 (Actor|GetActorOfClass "/Game/Button/BP_BUpgrade.BP_BUpgrade_C"))
                (Utilities|IsValid _returnvalue_7
                  (:Is%20Not%20Valid
                    (bind _asbpgi_oxygen_8 (Utilities|Casting|CastToBPGI_Oxygen (Game|GetGameInstance)))
                    (Variables|/Game/Tree/BPGI_Oxygen.BPGI_Oxygen_C|SetOxygen _asbpgi_oxygen_8 (- (Variables|/Game/Tree/BPGI_Oxygen.BPGI_Oxygen_C|GetOxygen _asbpgi_oxygen_8) (Variables|Default|GetPrice%20O2)))
                    (bind _returnvalue_8 (Actor|GetActorOfClass "/Game/Tree/BP_Tree3.BP_Tree3_C"))
                    (Actor|DestroyActor _returnvalue_8)
                    (Game|SpawnActorfromClass "/Game/Tree/BP_Tree4.BP_Tree4_C" (Math|Transform|MakeTransform (Variables|Default|GetLocation%20Spawn) "0, 0, 0" "1.000000,1.000000,1.000000") "Undefined" "MultiplyWithRoot" 0 0)
                    (Variables|Default|SetLevel%20Tree 5)
                    (Variables|Default|SetSpawn%20Upgrade%20Tree false))))))
          (elif (== (Variables|Default|GetLevel%20Tree) 5)
            (bind _asbpgi_oxygen_9 (Utilities|Casting|CastToBPGI_Oxygen (Game|GetGameInstance)))
            (if (>= (Variables|/Game/Tree/BPGI_Oxygen.BPGI_Oxygen_C|GetOxygen _asbpgi_oxygen_9) (Variables|Default|GetPrice%20O2))
              (bind _output_get_5 (Variables|Default|SetUpgrade? true))
              (if (and _output_get_5 (== (Variables|Default|GetSpawn%20Upgrade%20Tree) false))
                (CallFunction|UpgradeTree)
                (else
                  (bind _returnvalue_9 (Actor|GetActorOfClass "/Game/Button/BP_BUpgrade.BP_BUpgrade_C"))
                  (Utilities|IsValid _returnvalue_9
                    (:Is%20Not%20Valid
                      (bind _asbpgi_oxygen_10 (Utilities|Casting|CastToBPGI_Oxygen (Game|GetGameInstance)))
                      (Variables|/Game/Tree/BPGI_Oxygen.BPGI_Oxygen_C|SetOxygen _asbpgi_oxygen_10 (- (Variables|/Game/Tree/BPGI_Oxygen.BPGI_Oxygen_C|GetOxygen _asbpgi_oxygen_10) (Variables|Default|GetPrice%20O2)))
                      (bind _returnvalue_10 (Actor|GetActorOfClass "/Game/Tree/BP_Tree4.BP_Tree4_C"))
                      (Actor|DestroyActor _returnvalue_10)
                      (Game|SpawnActorfromClass "/Game/Tree/BP_Tree5.BP_Tree5_C" (Math|Transform|MakeTransform (Variables|Default|GetLocation%20Spawn) "0, 0, 0" "1.000000,1.000000,1.000000") "Undefined" "MultiplyWithRoot" 0 0)
                      (Variables|Default|SetLevel%20Tree 6)
                      (Variables|Default|SetSpawn%20Upgrade%20Tree false))))))
            (elif (== (Variables|Default|GetLevel%20Tree) 6)
              (CallFunction|BeliPohonBaru)
              (if (and (== (Variables|Default|GetCan%20Buy%20a%20Tree?) true) (== (Variables|Default|GetSpawn%20New%20Tree) false))
                (Game|SpawnActorfromClass "/Game/Button/BP_BNewTree.BP_BNewTree_C" (Math|Transform|MakeTransform "1360.000000,22410.000000,120.000000" "0, 0, 0" "1.000000,1.000000,1.000000") "Undefined" "MultiplyWithRoot" 0 0)
                (Variables|Default|SetSpawn%20New%20Tree true)
                (else
                  (bind _returnvalue_11 (Actor|GetActorOfClass "/Game/Button/BP_BNewTree.BP_BNewTree_C"))
                  (Utilities|IsValid _returnvalue_11
                    (:Is%20Not%20Valid
                      (if (not (== (Variables|Default|GetBuy) false))
                        (Variables|Default|SetCan%20Buy%20a%20Tree? false)
                        (Variables|Default|SetSpawn%20New%20Tree false)
                        (bind _returnvalue_12 (Actor|GetActorOfClass "/Game/Lahan/BP_LahanBelakang.BP_LahanBelakang_C"))
                        (Default|NewTree _returnvalue_12)
                        (Utilities|FlowControl|DelayUntilNextTick)
                        (bind _returnvalue_13 (Actor|GetActorOfClass "/Game/Tree/BP_Tree5.BP_Tree5_C"))
                        (Actor|DestroyActor _returnvalue_13)
                        (Variables|Default|SetBuy false)
                        (Game|SpawnActorfromClass "/Game/Tree/BP_DeadTree.BP_DeadTree_C" (Math|Transform|MakeTransform (Variables|Default|GetLocation%20Spawn) "0, 0, 0" "1.000000,1.000000,1.000000") "Undefined" "MultiplyWithRoot" 0 0)
                        (Variables|Default|SetLevel%20Tree 1)))))))))))))

(fn ConstructionScript)