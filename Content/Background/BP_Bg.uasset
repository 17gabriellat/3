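; BP_Bg is a background controller that alternates day (Siang) and night (Malam) backdrops in an endless cycle.
; On BeginPlay it caches the BP_LahanUtama actor and starts ChangeTime, which spawns each backdrop actor at a fixed offset from that actor's Plane.
; Each backdrop lasts for a fixed delay before being destroyed, then ChangeTime calls itself to repeat the loop.
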(event Custom|Change%20Time
  ;[1 1 1] Change BG Siang Malam
  (bind _returnvalue (Game|SpawnActorfromClass "/Game/Background/BP_Siang.BP_Siang_C" (Math|Transform|MakeTransform (+ (Transformation|GetWorldLocation (Variables|/Game/Lahan/BP_LahanUtama.BP_LahanUtama_C|GetPlane (Variables|Default|GetRefLahan))) "500.000000,-10.000000,210.000000") "0, 0, 0" "1.000000,1.000000,1.000000") "Undefined" "MultiplyWithRoot" 0 0))
  (Utilities|FlowControl|Delay 1e+01)
  (Actor|DestroyActor _returnvalue)
  (bind _returnvalue_2 (Game|SpawnActorfromClass "/Game/Background/BP_Malam.BP_Malam_C" (Math|Transform|MakeTransform (+ (Transformation|GetWorldLocation (Variables|/Game/Lahan/BP_LahanUtama.BP_LahanUtama_C|GetPlane (Variables|Default|GetRefLahan))) "500.000000,-10.000000,210.000000") "0, 0, 0" "1.000000,1.000000,1.000000") "Undefined" "MultiplyWithRoot" 0 0))
  (Utilities|FlowControl|Delay 1e+01)
  (Actor|DestroyActor _returnvalue_2)
  (CallFunction|ChangeTime))

(event EventBeginPlay
  (bind _returnvalue (Actor|GetActorOfClass "/Game/Lahan/BP_LahanUtama.BP_LahanUtama_C"))
  (Variables|Default|SetRefLahan _returnvalue)
  (CallFunction|ChangeTime))

(fn ConstructionScript)