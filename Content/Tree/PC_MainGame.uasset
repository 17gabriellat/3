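; PC_MainGame is a player controller that turns tap input into a Count call on the tree actor.
; On BeginPlay it adds the IMC_Inputan Enhanced Input mapping context and shows the mouse cursor, provided the input subsystem is valid.
; When IA_Tap starts, it looks up BP_Tree by class and calls Count, regardless of where the tap lands.
; An under-cursor trace cast to BP_Tree is left unconnected.
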(event Input|EnhancedActionEvents|EnhancedInputActionIA_Tap
  (params (ActionValue :type Float%20%28double-precision%29) (ElapsedSeconds :type Float%20%28double-precision%29) (TriggeredSeconds :type Float%20%28double-precision%29) (InputAction :type Input%20Action%20Object%20Reference :default "/Game/Input/Input_Action/IA_Tap.IA_Tap"))
  (:Started
    (bind _returnvalue (Actor|GetActorOfClass "/Game/Tree/BP_Tree.BP_Tree_C"))
    (Default|Count++ _returnvalue)))

(event EventBeginPlay
  (bind _returnvalue (PlayerController|LocalPlayerSubsystems|GetEnhancedInputLocalPlayerSubsystem))
  (Utilities|IsValid _returnvalue
    (:Is%20Valid
      (Input|AddMappingContext _returnvalue "/Game/Input/IMC_Inputan.IMC_Inputan" 0 "(bIgnoreAllPressedKeysUntilRelease=True,bForceImmediately=False,bNotifyUserSettings=False)")
      (Variables|Default|SetbShowMouseCursor true))))

(event EventTick
  (params (DeltaSeconds :type Float%20%28single-precision%29)))

(fn ConstructionScript)