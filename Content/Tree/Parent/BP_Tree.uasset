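; BP_Tree is a parent tree Blueprint that awards oxygen for player taps.
; Count++ handles screen taps by adding TapOxygen to the Oxygen total in BPGI_Oxygen, the Game Instance.
; SpecialCount handles taps directly on the tree and adds double TapOxygen.
; Both events print the new total; BeginPlay and the construction script are empty, and tap detection is not in this graph.
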(event Custom|Count++
  ;[1 1 1] Hasil Oksigen dari Tap di Screen
  (bind _asbpgi_oxygen (Utilities|Casting|CastToBPGI_Oxygen (Game|GetGameInstance)))
  (bind _output_get (Variables|/Game/Tree/BPGI_Oxygen.BPGI_Oxygen_C|SetOxygen _asbpgi_oxygen (+ (Variables|/Game/Tree/BPGI_Oxygen.BPGI_Oxygen_C|GetOxygen _asbpgi_oxygen) (Variables|Default|GetTap%20Oxygen))))
  (Development|PrintString (Utilities|String|ToString(Float) _output_get)))

(event Custom|SpecialCount
  ;[1 1 1] Hasil Oksigen dari Tap Langsung Pohon
  (bind _asbpgi_oxygen (Utilities|Casting|CastToBPGI_Oxygen (Game|GetGameInstance)))
  (bind _output_get (Variables|/Game/Tree/BPGI_Oxygen.BPGI_Oxygen_C|SetOxygen _asbpgi_oxygen (+ (Variables|/Game/Tree/BPGI_Oxygen.BPGI_Oxygen_C|GetOxygen _asbpgi_oxygen) (* (Variables|Default|GetTap%20Oxygen) 2.0))))
  (Development|PrintString (Utilities|String|ToString(Float) _output_get)))

(event EventBeginPlay)

(fn ConstructionScript)